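; BP_HeroCharacter is the player hero character Blueprint, handling hit feedback and opening the pause screen.
; On damage, a timeline drives the HitFxSwitch material parameter on the body mesh and, if valid, the currently equipped weapon's mesh from the hero combat component.
; The pause input asynchronously loads the pause screen widget class, then creates it and adds it to the viewport.
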(event Input|EnhancedActionEvents|EnhancedInputActionIA_PauseMenu
  (params (ActionValue :type Boolean) (ElapsedSeconds :type Float%20%28double-precision%29) (TriggeredSeconds :type Float%20%28double-precision%29) (InputAction :type Input%20Action%20Object%20Reference :default "/Game/PlayerCharacter/Input/Actions/IA_PauseMenu.IA_PauseMenu"))
  (:Started
    (bind _class (Utilities|AsyncLoadClassAsset "/Game/Widgets/GameModeWidgets/WBP_PauseScreen.WBP_PauseScreen_C")
      (:Completed
        (bind _asuser_widget (Utilities|Casting|CastToUserWidgetClass _class))
        (bind _returnvalue (UserInterface|CreateWidget _asuser_widget))
        (UserInterface|Viewport|AddtoViewport _returnvalue 0)))))

(event EventOnDamageTaken
  (params (DamageAmount :type Float%20%28single-precision%29) (DamageInstigator :type Actor%20Object%20Reference))
  (bind _herocombatcomponent (Variables|Default|GetHeroCombatComponent))
  (bind _returnvalue (Class|HeroCombatComponent|GetHeroCurrentEquippedWeapon _herocombatcomponent))
  (bind _weaponmesh (Variables|/Script/GodsentAvenger.GodsentWeaponBase|GetWeaponMesh _returnvalue))
  (bind _materialflash (Timeline|TL_HitFlash PlayFromStart)
    (:Update
      (Rendering|Material|SetScalarParameterValueonMaterials (Variables|Character|GetMesh) "HitFxSwitch" _materialflash)
      (Utilities|IsValid _weaponmesh
        (:Is%20Valid
          (Rendering|Material|SetScalarParameterValueonMaterials _weaponmesh "HitFxSwitch" _materialflash))))))

(fn ConstructionScript)
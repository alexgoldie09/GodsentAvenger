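; Base enemy character Blueprint that drives spawn, hit and death visuals on the body meshes and equipped weapon.
; On BeginPlay it plays a random entry montage while a reversed timeline animates DissolveAmount; damage triggers a HitFxSwitch flash.
; Death freezes animation, disables capsule collision, clears UI widgets, async-loads an edge-colored Niagara effect, dissolves, then destroys weapon and actor.
; Timelines feed a helper that sets material parameters on every static and skeletal mesh component.
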(event EventBeginPlay
  (bind _enemycombatcomponent (Variables|Default|GetEnemyCombatComponent))
  (bind _entrymontagestoplay (Variables|Default|GetEntryMontagesToPlay))
  (bind _returnvalue (Class|PawnCombatComponent|GetCharacterCurrentEquippedWeapon _enemycombatcomponent))
  (Utilities|FlowControl|Sequence
    (:then_0
      (Components|Timeline|SetPlayRate (Variables|Default|GetEntryRestoreTimeline) (/ 1.0 (Variables|Default|GetTotalEntryRestoreTime)))
      (bind _normalizedfloattrack (Timeline|EntryRestoreTimeline ReverseFromEnd)
        (:Update
          ;[0.15 0.04568 0.02867 0.5] DissolveWeapon (if valid) and DissolveMesh
          (CallFunction|SetVisualMeshesScalarParameter "DissolveAmount" _normalizedfloattrack)
          (if (Variables|Default|GetbHasWeapon)
            (Utilities|IsValid _returnvalue
              (:Is%20Valid
                (Rendering|Material|SetScalarParameterValueonMaterials (Variables|/Script/GodsentAvenger.GodsentWeaponBase|GetWeaponMesh _returnvalue) "DissolveAmount" _normalizedfloattrack)))))))
    (:then_1
      (if (Utilities|Array|IsNotEmpty _entrymontagestoplay)
        (Animation|PlayAnimMontage (.OutItem (Utilities|Array|Random _entrymontagestoplay)) 1.0 "None")))))

(event EventOnEnemyDied
  (params (DissolveNiagaraSystem :type Niagara%20System%20Soft%20Object%20Reference))
  (bind _mesh (CallFunction|GetDissolveMesh))
  (bind _enemycombatcomponent (Variables|Default|GetEnemyCombatComponent))
  (bind _enemycombatcomponent_2 (Variables|Default|GetEnemyCombatComponent))
  (bind _returnvalue (Class|PawnCombatComponent|GetCharacterCurrentEquippedWeapon _enemycombatcomponent_2))
  (bind _returnvalue_2 (Class|PawnCombatComponent|GetCharacterCurrentEquippedWeapon _enemycombatcomponent))
  (Utilities|FlowControl|Sequence
    (:then_0
      (Variables|/Script/Engine.SkeletalMeshComponent|SetbPauseAnims (Variables|Character|GetMesh) true)
      (Collision|SetCollisionEnabled (Variables|Default|GetCapsuleComponent) "NoCollision"))
    (:then_1
      (Class|EnemyUIComponent|RemoveEnemyDrawnWidgetsifAny (Variables|Default|GetEnemyUIComponent)))
    (:then_2
      (bind _object (Utilities|AsyncLoadAsset DissolveNiagaraSystem)
        (:Completed
          (bind _asniagara_system (Utilities|Casting|CastToNiagaraSystem _object))
          (bind _returnvalue_3 (Niagara|SpawnSystemAttached _asniagara_system _mesh "None" "0, 0, 0" "0, 0, 0" "KeepRelativeOffset" true))
          (bind _returnvalue_4 (Rendering|Material|CreateDynamicMaterialInstance _mesh 0 (Rendering|Material|GetMaterial _mesh 0) "None" :!class /Script/Engine.PrimitiveComponent))
          (bind _returnvalue_5 (Rendering|Material|GetVectorParameterValue _returnvalue_4 "DissolveEdgeColor" :!class /Script/Engine.MaterialInstanceDynamic))
          (Niagara|SetNiagaraVariable(LinearColor) _returnvalue_3 "DissolveParticleColor" _returnvalue_5)
          (Components|Timeline|SetPlayRate (Variables|Default|GetDissolveTimeline) (/ 1.0 (Variables|Default|GetTotalDissolveTime)))
          (bind _normalizedfloattrack (Timeline|DissolveTimeline PlayFromStart)
            (:Update
              ;[0.15 0.04568 0.02867 0.5] DissolveWeapon (if valid) and DissolveMesh
              (CallFunction|SetVisualMeshesScalarParameter "DissolveAmount" _normalizedfloattrack)
              (if (Variables|Default|GetbHasWeapon)
                (Utilities|IsValid _returnvalue_2
                  (:Is%20Valid
                    (Rendering|Material|SetScalarParameterValueonMaterials (Variables|/Script/GodsentAvenger.GodsentWeaponBase|GetWeaponMesh _returnvalue_2) "DissolveAmount" _normalizedfloattrack)))))
            (:Finished
              ;[0.15 0.1403 0.02461 0.5] DestroyWeapon (if valid) and DestroyActor
              (if (Variables|Default|GetbHasWeapon)
                (Utilities|IsValid _returnvalue
                  (:Is%20Valid
                    (Actor|DestroyActor _returnvalue))))
              (Actor|DestroyActor))))))))

(event EventOnDamageTaken
  (params (DamageAmount :type Float%20%28single-precision%29) (DamageInstigator :type Actor%20Object%20Reference))
  (bind _enemycombatcomponent (Variables|Default|GetEnemyCombatComponent))
  (bind _returnvalue (Class|PawnCombatComponent|GetCharacterCurrentEquippedWeapon _enemycombatcomponent))
  (bind _weaponmesh (Variables|/Script/GodsentAvenger.GodsentWeaponBase|GetWeaponMesh _returnvalue))
  (bind _materialflash (Timeline|Timeline PlayFromStart)
    (:Update
      (CallFunction|SetVisualMeshesScalarParameter "HitFxSwitch" _materialflash)
      (if (Variables|Default|GetbHasWeapon)
        (Utilities|IsValid _weaponmesh
          (:Is%20Valid
            (Rendering|Material|SetScalarParameterValueonMaterials _weaponmesh "HitFxSwitch" _materialflash)))))))

(fn ConstructionScript)

(fn GetVisualMeshes
  (Utilities|Array|Clear (LocalVariables|GetCachedMeshes))
  (for _array_element (Actor|GetComponentsByClass "/Script/Engine.StaticMeshComponent")
    (Utilities|Array|Add (LocalVariables|GetCachedMeshes) _array_element))
  (for _array_element_2 (Actor|GetComponentsByClass "/Script/Engine.SkeletalMeshComponent")
    (Utilities|Array|Add (LocalVariables|GetCachedMeshes) _array_element_2))
  (return (LocalVariables|GetCachedMeshes)))

(fn SetVisualMeshesScalarParameter
  (params (Name :type Name) (Value :type Float%20%28double-precision%29))
  (for _array_element (CallFunction|GetVisualMeshes)
    (Rendering|Material|SetScalarParameterValueonMaterials _array_element Name Value)))

(fn GetDissolveMesh
  (return (Variables|Character|GetMesh)))